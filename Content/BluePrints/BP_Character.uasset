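; BP_Character is a character Blueprint that lets the player grab interactables and throw held objects.
; Grab input throws the held object, or, if none is held and an interactable is found, disables pawn movement and extends TDHandIK toward it.
; BeginPlay initializes the character with its holster and sphere grab region, then the hand IK with the right hand's anim instance, grab curve and IK target.
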(event `InputAction|Grab`
  (params (Key :type "Key Structure"))
  (:`Pressed`
    (bind _success (`self.GetHeldObject`))
    (if _success
      (`self.Throw` (`self.ThrowStrength`))
      (else
        ;[1 1 1] Grab
        (bind (_success_2 _interactable) (`self.GetInteractable`))
        (if _success_2
          (set `TD_PawnMovementComponent.CanMove` false (`self.TD_PawnMovement`))
          (`TD_HandIKComponent.Extend` (`self.TD_HandIK`) (`Actor.RootComponent` _interactable))
          (`KismetSystemLibrary.PrintString` "Extended!!"))))))

(event `self.ReceiveBeginPlay`
  (`|ExecutionSequence`
    (:`then_0`
      ;[1 1 1] TD_Character Init
      (`self.Init` (`self.HolsterComp`) (`self.Sphere_GrabRegion`)))
    (:`then_1`
      ;[1 1 1] TD_Hand_IK Init
      (bind _ashand_abp (cast `/Game/Models/Hand/hand_ABP` (`SkeletalMeshComponent.GetAnimInstance` (`self.Hand_R`))))
      (`TD_HandIKComponent.Init` (`self.TD_HandIK`) _ashand_abp "/Game/BluePrints/GrabCurve.GrabCurve" (`self.Hand_IK_Target_R`)))))

(fn `UserConstructionScript`)