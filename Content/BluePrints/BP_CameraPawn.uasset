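; Camera pawn that snaps to a CameraTarget on BeginPlay and moves its Scene component to follow that target every tick.
; Zoom inputs lengthen or shorten the SpringArm by ZoomSpeed, with no clamping.
; Horizontal input yaws the pawn while a click is held or the stick moves, with holds confirmed by a short delayed key check.
; Vertical pitch logic exists but is disconnected, so it never runs.
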(event `self.ReceiveTick`
  (params (DeltaSeconds :type "Float (single-precision)"))
  (`SceneComponent.K2_SetWorldLocation` (`self.Scene`) (`SceneComponent.K2_GetComponentLocation` (`Actor.RootComponent` (`self.CameraTarget`))) false false))

(event `self.ReceiveBeginPlay`
  ;[1 1 1] BeginPlay
  (`self.K2_SetActorLocation` (`self.K2_GetActorLocation` (`self.CameraTarget`))))

(event `OnClickPressed`
  (params (Key :type "Key Structure" :default "None"))
  ;[1 1 1] Click
  (`KismetSystemLibrary.Delay` 0.1)
  (set `self.bClickHeld` (`PlayerController.IsInputKeyDown` (`GameplayStatics.GetPlayerController` 0) Key)))

(event `OnClickReleased`
  (params (Key :type "Key Structure" :default "None"))
  ;[1 1 1] Click
  (set `self.bClickHeld` false))

(event `OnZoomIn`
  ;[1 1 1] Zoom
  (`self.Zoom` (`self.ZoomSpeed`)))

(event `OnZoomOut`
  ;[1 1 1] Zoom
  (`self.Zoom` (* -1 (`self.ZoomSpeed`))))

(event `OnRotateHorz`
  (params (`Axiz Value` :type "Float (double-precision)") (`axis value stick` :type "Float (double-precision)"))
  ;[1 1 1] Rotate
  (if (or (`self.bClickHeld`) (!= `axis value stick` 0.0))
    (`self.K2_AddActorWorldRotation` (`KismetMathLibrary.MakeRotator` 0.0 0.0 (* `Axiz Value` (`self.RotationSpeed`))))))

(event `OnRotateVert`
  (params (`Axis Value` :type "Float (double-precision)") (`Axis Value Stick` :type "Float (double-precision)"))
  ;[1 1 1] Rotate
)

(fn `UserConstructionScript`
  (locals (NewLocalVar_0 :type "SpringArmComponent Object Reference") (NewLocalVar_1 :type "Float (double-precision)" :default 0.0) (NewLocalVar_2 :type "Float (double-precision)" :default 0.0)))

(fn `Zoom`
  (params (ZoomSpeed :type "Float (double-precision)"))
  (bind _springarm (`self.SpringArm`))
  (set `SpringArmComponent.TargetArmLength` (+ (`SpringArmComponent.TargetArmLength` _springarm) ZoomSpeed) _springarm))