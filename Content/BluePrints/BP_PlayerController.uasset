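; Player controller that drives a character with camera-relative movement and relays input to a separate BP_CameraPawn found in the level at BeginPlay.
; Move axes feed ApplyMovement and ApplyRotations, which use the camera manager's forward (flattened) and right vectors to move the character and face it along its input.
; Click, zoom and rotate inputs go to the camera pawn, and Grab to the character.
; Uncalled debug helpers draw input and facing arrows.
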(event `self.ReceiveBeginPlay`
  ;[1 1 1] Init
  (`|ExecutionSequence`
    (:`then_0`
      (set `self.bShowMouseCursor` true))
    (:`then_1`
      (bind _ascharacter (cast `Character` (`self.CharacterPawn`)))
      (set `self.CharacterObj` _ascharacter))
    (:`then_2`
      (bind _outactors (`GameplayStatics.GetAllActorsOfClass` "/Game/BluePrints/BP_CameraPawn.BP_CameraPawn_C"))
      (bind _asbp_camera_pawn (cast `/Game/BluePrints/BP_CameraPawn` (`|GetArrayItem` _outactors)))
      (set `self.BP_Camera` _asbp_camera_pawn))))

(event `InputAxis|MoveForwards`
  (params (AxisValue :type "Float (single-precision)"))
  (set `self.forwardInput` AxisValue)
  (`self.applyMovement` :!label _label)
  (`self.applyRotations`))

(event `InputAxis|MoveRight`
  (params (AxisValue :type "Float (single-precision)"))
  (set `self.rightInput` AxisValue)
  (goto _label))

(event `InputAction|Grab`
  (params (Key :type "Key Structure"))
  (:`Pressed`
    (`TD_Character.Grab` (`self.BP_Character`))))

(event `InputAction|Click`
  (params (Key :type "Key Structure"))
  (bind _bp_camera (`self.BP_Camera`))
  ;[1 1 1] Click
  (:`Pressed`
    (`/Game/BluePrints/BP_CameraPawn.OnClickPressed` _bp_camera Key))
  (:`Released`
    (`/Game/BluePrints/BP_CameraPawn.OnClickReleased` _bp_camera Key)))

(event `InputAction|ZoomIn`
  (params (Key :type "Key Structure"))
  ;[1 1 1] Zoom
  (:`Pressed`
    (`/Game/BluePrints/BP_CameraPawn.OnZoomIn` (`self.BP_Camera`))))

(event `InputAction|ZoomOut`
  (params (Key :type "Key Structure"))
  ;[1 1 1] Zoom
  (:`Pressed`
    (`/Game/BluePrints/BP_CameraPawn.OnZoomOut` (`self.BP_Camera`))))

(event `InputAxis|RotateHorz`
  (params (AxisValue :type "Float (single-precision)"))
  ;[1 1 1] Rotate
  (`/Game/BluePrints/BP_CameraPawn.OnRotateHorz` (`self.BP_Camera`) AxisValue (`self.GetInputAxisValue`)))

(event `InputAxis|RotateVert`
  (params (AxisValue :type "Float (single-precision)"))
  ;[1 1 1] Rotate
  (`/Game/BluePrints/BP_CameraPawn.OnRotateVert` (`self.BP_Camera`) AxisValue (`self.GetInputAxisValue`)))

(fn `applyMovement`
  (bind _bp_character (`self.BP_Character`))
  (`|ExecutionSequence`
    (:`then_0`
      (bind _cameraforward (`self.GetCameraForward`))
      (`Pawn.AddMovementInput` _bp_character _cameraforward (`self.forwardInput`) false))
    (:`then_1`
      (bind _cameraright (`self.GetCameraRight`))
      (`Pawn.AddMovementInput` _bp_character _cameraright (`self.rightInput`) false))))

(fn `applyRotations`
  (`|ExecutionSequence`
    (:`then_0`
      (bind _cameraforward (`self.GetCameraForward`)))
    (:`then_1`
      (bind _cameraright (`self.GetCameraRight`))))
  (bind _output_get (set `self.inputVector` (`KismetMathLibrary.Normal` (+ (* _cameraforward (`self.forwardInput`)) (* _cameraright (`self.rightInput`))))))
  (if (> (`KismetMathLibrary.VSize` _output_get) 0.0)
    (`self.K2_SetActorRotation` (`self.BP_Character`) (`KismetMathLibrary.Conv_VectorToRotator` _output_get) false)))

(fn `drawForward`
  (bind _characterpawn (`self.CharacterPawn`))
  (`self.DrawVectorFrom` _characterpawn (`self.GetActorForwardVector` _characterpawn) (struct :`R` 1.0 :`G` 0.316556 :`A` 1.0)))

(fn `drawInput`
  (`self.DrawVectorFrom` (`self.CharacterPawn`) (`self.inputVector`) (struct :`R` 0.832854 :`B` 1.0 :`A` 1.0)))

(fn `GetCameraForward`
  (returns (cameraForward :type "Vector Structure"))
  (bind (_returnvalue_x _returnvalue_y) (`KismetMathLibrary.BreakVector` (`self.GetActorForwardVector` (`GameplayStatics.GetPlayerCameraManager` 0))))
  (return (`KismetMathLibrary.Normal` (`KismetMathLibrary.MakeVector` _returnvalue_x _returnvalue_y))))

(fn `GetCameraRight`
  (returns (cameraRight :type "Vector Structure"))
  (return (`KismetMathLibrary.Normal` (`self.GetActorRightVector` (`GameplayStatics.GetPlayerCameraManager` 0)))))

(fn `UserConstructionScript`)