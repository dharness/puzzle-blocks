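; Actor that keeps a Cube on the surface between a Target component and a Sphere component, oriented away from the Sphere's center.
; Each Tick aligns the Cube's Z axis to the normalized Sphere-to-Target direction.
; A complex visibility trace from Target to Sphere, which can hit the actor itself, moves the Cube to the impact.
; Debug arrows show that direction and the Cube's up vector.
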(event `self.ReceiveBeginPlay`)

(event `self.ReceiveTick`
  (params (DeltaSeconds :type "Float (single-precision)"))
  (bind _returnvalue (`self.K2_GetActorLocation`))
  (bind _cube (`self.Cube`))
  (bind _returnvalue_2 (`SceneComponent.K2_GetComponentLocation` _cube))
  (bind _returnvalue_3 (`KismetMathLibrary.Normal` (- (`SceneComponent.K2_GetComponentLocation` (`self.Target`)) (`SceneComponent.K2_GetComponentLocation` (`self.Sphere`)))))
  (`|ExecutionSequence`
    (:`then_0`
      (`KismetSystemLibrary.DrawDebugArrow` _returnvalue (+ _returnvalue (* _returnvalue_3 150.0)) 0.0 (struct :`R` 0.92163 :`G` 0.097376 :`B` 1.0 :`A` 1.0) 0.1 2.0)
      (`SceneComponent.K2_SetWorldRotation` (`self.Cube`) (`KismetMathLibrary.MakeRotFromZ` _returnvalue_3) false false)
      (bind (_outhit _returnvalue_4) (`KismetSystemLibrary.LineTraceSingle` :`Start` (`SceneComponent.K2_GetComponentLocation` (`self.Target`)) :`End` (`SceneComponent.K2_GetComponentLocation` (`self.Sphere`)) :`TraceChannel` "TraceTypeQuery1" :`bTraceComplex` true :`DrawDebugType` "ForOneFrame" :`bIgnoreSelf` false))
      (if _returnvalue_4
        (`SceneComponent.K2_SetWorldLocation` (`self.Cube`) (`.Location` (`GameplayStatics.BreakHitResult` _outhit)) false false)))
    (:`then_1`
      (`KismetSystemLibrary.DrawDebugArrow` _returnvalue_2 (+ _returnvalue_2 (* (`SceneComponent.GetUpVector` _cube) 150.0)) 0.0 (struct :`G` 0.066144 :`B` 1.0 :`A` 1.0) 0.1 2.0))))

(fn `UserConstructionScript`)