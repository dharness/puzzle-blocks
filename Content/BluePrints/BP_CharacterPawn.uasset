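; Player character pawn that forwards click, zoom and rotate input to a separate camera pawn and holds logic for grabbing and throwing objects.
; Hand-region overlaps track BPI_Interactable actors, selecting the first as the grab target.
; Grab attaches it to a holster without pawn collision; throw launches it forward with a debug trajectory, restoring collision on capsule exit.
; The grab/throw trigger is disconnected, as is a floor material-parameter update.
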(event `self.ReceiveTick`
  (params (DeltaSeconds :type "Float (single-precision)")))

(event `self.hands_grab_region.OnComponentBeginOverlap`
  (params (OverlappedComponent :type "PrimitiveComponent Object Reference") (OtherActor :type "Actor Object Reference") (OtherComp :type "PrimitiveComponent Object Reference") (OtherBodyIndex :type Integer) (bFromSweep :type Boolean) (SweepResult :type "HitResult Structure (by ref)"))
  ;[1 1 1] Grab
  (`self.UpdateInteractables` :!label _label))

(event `self.hands_grab_region.OnComponentEndOverlap`
  (params (OverlappedComponent :type "PrimitiveComponent Object Reference") (OtherActor :type "Actor Object Reference") (OtherComp :type "PrimitiveComponent Object Reference") (OtherBodyIndex :type Integer))
  ;[1 1 1] Grab
  (goto _label))

(event `self.CapsuleComponent.OnComponentEndOverlap`
  (params (OverlappedComponent :type "PrimitiveComponent Object Reference") (OtherActor :type "Actor Object Reference") (OtherComp :type "PrimitiveComponent Object Reference") (OtherBodyIndex :type Integer))
  (if (`self.hasThrown`)
    (`KismetSystemLibrary.PrintString` (`KismetSystemLibrary.GetDisplayName` OtherActor))
    (set `self.hasThrown` false)
    (`PrimitiveComponent.SetCollisionProfileName` (`self.GetComponentByClass` OtherActor "/Script/Engine.StaticMeshComponent") "BlockAll")))

(event `InputAction|Click`
  (params (Key :type "Key Structure"))
  (bind _bp_camerapawn (`self.BP_CameraPawn`))
  ;[1 1 1] Click
  (:`Pressed`
    (`/Game/BluePrints/BP_CameraPawn.OnClickPressed` _bp_camerapawn Key))
  (:`Released`
    (`/Game/BluePrints/BP_CameraPawn.OnClickReleased` _bp_camerapawn Key)))

(event `InputAction|ZoomIn`
  (params (Key :type "Key Structure"))
  ;[1 1 1] Zoom
  (:`Pressed`
    (`/Game/BluePrints/BP_CameraPawn.OnZoomIn` (`self.BP_CameraPawn`))))

(event `InputAction|ZoomOut`
  (params (Key :type "Key Structure"))
  ;[1 1 1] Zoom
  (:`Pressed`
    (`/Game/BluePrints/BP_CameraPawn.OnZoomOut` (`self.BP_CameraPawn`))))

(event `InputAxis|RotateHorz`
  (params (AxisValue :type "Float (single-precision)"))
  ;[1 1 1] Rotate
  (`/Game/BluePrints/BP_CameraPawn.OnRotateHorz` (`self.BP_CameraPawn`) AxisValue (`self.GetInputAxisValue`)))

(event `InputAxis|RotateVert`
  (params (AxisValue :type "Float (single-precision)"))
  ;[1 1 1] Rotate
  (`/Game/BluePrints/BP_CameraPawn.OnRotateVert` (`self.BP_CameraPawn`) AxisValue (`self.GetInputAxisValue`)))

(fn `Grab Object`
  (bind _interactableobject (`self.interactableObject`))
  (bind _returnvalue (`self.GetComponentByClass` _interactableobject "/Script/Engine.StaticMeshComponent"))
  (`/Engine/EditorBlueprintResources/StandardMacros.IsValid` _interactableobject
    (:`Is Valid`
      (`PrimitiveComponent.SetSimulatePhysics` _returnvalue false)
      (`self.K2_AttachToComponent` _interactableobject (`self.holster`) "None" "SnapToTarget" "SnapToTarget" "KeepWorld" false)
      (set `self.heldObject` _interactableobject)
      (`PrimitiveComponent.SetCollisionProfileName` _returnvalue "NoPawn"))))

(fn `Throw Object`
  (params (toThrow :type "Actor Object Reference"))
  (locals (objectToThrow :type "Actor Object Reference"))
  (bind _returnvalue (`self.GetComponentByClass` toThrow "/Script/Engine.StaticMeshComponent"))
  (bind _objecttothrow (`local.objectToThrow`))
  (bind _returnvalue_2 (* (`self.GetActorForwardVector`) 500.0))
  (bind _output_get (set `local.objectToThrow` toThrow))
  (`SceneComponent.K2_DetachFromComponent` (`Actor.RootComponent` _output_get) "KeepWorld" "KeepWorld" "KeepWorld" true)
  (`PrimitiveComponent.SetSimulatePhysics` _returnvalue true)
  (`PrimitiveComponent.SetPhysicsLinearVelocity` _returnvalue _returnvalue_2 true "None")
  (`|ExecutionSequence`
    (:`then_0`
      (set `self.hasThrown` true)
      (set `self.heldObject` null))
    (:`then_1`
      (`GameplayStatics.Blueprint_PredictProjectilePath_ByTraceChannel` (`self.K2_GetActorLocation` _objecttothrow) _returnvalue_2 true 1.0 "ECC_Visibility" false (`|MakeArray` _objecttothrow self :!type "Actor Object Reference") "ForDuration" 5.0))))

(fn `UpdateInteractables`
  (locals (tmpArray :type "Array of Actor Object Reference"))
  (bind _tmparray (`local.tmpArray`))
  (for _array_element (`PrimitiveComponent.GetOverlappingActors` (`self.hands_grab_region`) null)
    (if (`KismetSystemLibrary.DoesImplementInterface` _array_element "/Game/BluePrints/BPI_Interactable.BPI_Interactable_C")
      (`KismetArrayLibrary.Array_Add` _tmparray _array_element)))
  (bind _output_get (set `self.interactableObjects` _tmparray))
  (bind _output (`|GetArrayItem` _output_get))
  (`/Engine/EditorBlueprintResources/StandardMacros.IsValid` _output
    (:`Is Valid`
      (set `self.interactableObject` _output))))

(fn `UserConstructionScript`)